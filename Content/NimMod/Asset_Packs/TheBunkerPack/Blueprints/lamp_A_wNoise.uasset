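; Lamp Blueprint from the bunker pack whose point light flickers randomly in color.
; Every Tick sets PointLight1 to a random linear blend between BlinkColor and BlinkColor2, with no timer or smoothing, so the flicker rate follows the frame rate.
; The construction script applies the same random blend, so the light already has a mixed color when constructed.
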(event `self.ReceiveTick`
  (params (DeltaSeconds :type "Float (single-precision)"))
  (`LightComponent.SetLightColor` (`self.PointLight1`) (`KismetMathLibrary.LinearColorLerp` (`self.blinkColor`) (`self.blinkColor2`) (`KismetMathLibrary.RandomFloatInRange` 0.0 1.0))))

(fn `UserConstructionScript`
  (`LightComponent.SetLightColor` (`self.PointLight1`) (`KismetMathLibrary.LinearColorLerp` (`self.blinkColor`) (`self.blinkColor2`) (`KismetMathLibrary.RandomFloatInRange` 0.0 1.0))))