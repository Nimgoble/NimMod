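; Urban city prop Blueprint that randomizes the material look of its static mesh each time play begins.
; The construction script creates a dynamic material instance on the mesh's first material slot.
; BeginPlay uses coin flips to set UCoord and VCoord to one of two half-step values, suggesting a four-quadrant texture atlas, and to switch the Lights parameter on or off.
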(event `self.ReceiveBeginPlay`
  (`MaterialInstanceDynamic.SetScalarParameterValue` (`self.DMI`) "UCoord" (`KismetMathLibrary.SelectFloat` 0.0 0.5 (`KismetMathLibrary.RandomBool`)))
  (`MaterialInstanceDynamic.SetScalarParameterValue` (`self.DMI`) "VCoord" (`KismetMathLibrary.SelectFloat` 0.0 0.5 (`KismetMathLibrary.RandomBool`)))
  (`MaterialInstanceDynamic.SetScalarParameterValue` (`self.DMI`) "Lights" (`KismetMathLibrary.SelectFloat` 0.0 1.0 (`KismetMathLibrary.RandomBool`))))

(fn `UserConstructionScript`
  (bind _returnvalue (`PrimitiveComponent.CreateDynamicMaterialInstance` (`self.StaticMesh1`) 0 null))
  (set `self.DMI` _returnvalue))