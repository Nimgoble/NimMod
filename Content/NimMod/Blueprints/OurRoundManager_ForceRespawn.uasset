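; Round manager that resets the level between rounds by force-respawning resettable actors and incrementing the round count.
; BeginPlay records every actor that passes ShouldReset.
; On HandleRestartRound, it sorts current actors against that list, spawning same-class replacements for recorded ones at their current transform and owner, then destroying the originals and any unrecorded resettable actors.
; Replacements become the next round's tracked set, with debug prints reporting counts and respawns.
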(event EventBeginPlay
  (CallFunction|GetLevelActors))

(event EventTick
  (params (DeltaSeconds :type Float%20%28single-precision%29)))

(event EventHandleRestartRound
  (CallFunction|RespawnActors))

(fn ConstructionScript)

(fn GetLevelActors
  (bind _currentroundactors (Variables|Default|GetCurrentRoundActors))
  (bind _outactors (Actor|GetAllActorsOfClass "/Script/Engine.Actor"))
  (for _array_element _outactors
    (bind _returnvalue (Class|RoundManager|ShouldReset _array_element))
    (if _returnvalue
      (Utilities|Array|Add _currentroundactors _array_element)))
  (Development|PrintText (Utilities|Text|FormatText "Current Round Actors after 'GetLevelActors': {0}" (Utilities|Text|ToText(Integer) (Utilities|Array|Length _currentroundactors)))))

(fn RespawnActors
  (bind _currentroundactors (Variables|Default|GetCurrentRoundActors))
  (bind _destroyactors (LocalVariables|GetdestroyActors))
  (bind _actorstorespawn (LocalVariables|GetactorsToRespawn))
  (bind _currentroundactors_2 (Variables|Default|GetCurrentRoundActors))
  (bind _actorstorespawn_2 (LocalVariables|GetactorsToRespawn))
  (bind _returnvalue (Utilities|Array|Length _actorstorespawn))
  (bind _returnvalue_2 (Utilities|Text|ToText(Integer) _returnvalue))
  (bind _result (Utilities|Text|FormatText "Actors To Respawn Count: {0}" _returnvalue_2))
  ;[1 1 1] See which of the actors in the level need to be respawned and which need to be destroyed.
  (bind _outactors (Actor|GetAllActorsOfClass "/Script/Engine.Actor"))
  (Development|PrintText (Utilities|Text|FormatText "All Actors count: {0}" (Utilities|Text|ToText(Integer) (Utilities|Array|Length _outactors))))
  (for _array_element _outactors
    (bind _returnvalue_3 (Class|RoundManager|ShouldReset _array_element))
    (if _returnvalue_3
      (if (Utilities|Array|ContainsItem _currentroundactors_2 _array_element)
        (Utilities|Array|Add _actorstorespawn _array_element)
        (Utilities|Array|RemoveItem _currentroundactors_2 _array_element)
        (else
          (Utilities|Array|Add (LocalVariables|GetdestroyActors) _array_element)))))
  (Development|PrintText _result)
  ;[1 1 1] Take care of any left-over actors from the beginning of the round that are no longer around
  (for _array_element_2 _currentroundactors_2
    (Utilities|IsValid _array_element_2
      (:Is%20Valid
        (bind _returnvalue_4 (Class|RoundManager|ShouldReset _array_element_2))
        (if _returnvalue_4
          (Utilities|Array|Add (LocalVariables|GetactorsToRespawn) _array_element_2)))
      (:Is%20Not%20Valid
        (Utilities|Array|Add (LocalVariables|GetdestroyActors) _array_element_2))))
  (Development|PrintText _result)
  ;[1 1 1] Respawn actors that need to be respawned
  (while (> (Utilities|Array|Length _actorstorespawn_2) 0)
    (bind _output_get (LocalVariables|SetCurrentRespawnActor (Utilities|Array|Get(acopy) _actorstorespawn_2)))
    (Utilities|IsValid _output_get
      (:Is%20Valid
        (Development|PrintText (Utilities|Text|FormatText "Respawning Actor: {0}" (Utilities|Text|ToText(String) (Utilities|GetObjectName _output_get))) true true "(R=0.000000,G=0.000000,B=0.000000,A=1.000000)")
        (bind _returnvalue_5 (Game|SpawnActorfromClass (Utilities|GetClass _output_get) (Transformation|GetActorTransform _output_get) "AlwaysSpawn" (Components|GetOwner _output_get) 0))
        (Utilities|Array|Add _currentroundactors _returnvalue_5)
        (if (Utilities|Array|ContainsItem _currentroundactors _output_get)
          (Utilities|Array|RemoveItem _currentroundactors _output_get))
        (Utilities|Array|Add (LocalVariables|GetdestroyActors) _output_get)
        (Utilities|Array|RemoveIndex (LocalVariables|GetactorsToRespawn)))
      (:Is%20Not%20Valid
        (Utilities|Array|RemoveIndex _actorstorespawn_2))))
  ;[1 1 1] Destroy the old actors
  (while (> (Utilities|Array|Length _destroyactors) 0)
    (bind _output_get_2 (LocalVariables|SetCurrentDestroyActor (Utilities|Array|Get(acopy) _destroyactors)))
    (Utilities|Array|RemoveIndex _destroyactors)
    (Utilities|IsValid _output_get_2
      (:Is%20Valid
        (Actor|DestroyActor _output_get_2))))
  ;[1 1 1] Increment the round count
  (Math|Integer|IncrementInt (Variables|Default|GetRoundCount)))