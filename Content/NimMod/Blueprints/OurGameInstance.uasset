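; Game instance Blueprint holding logic to update a dedicated server's listing on a Parse backend, though that chain is unconnected and never runs.
; The chain sets hard-coded Parse credentials, fills JSON with IP, name, map and player counts, then PUTs it to the ServerInstance object keyed by DedicatedServerID.
; Completion and failure events print the response.
; The debug printout swaps current and maximum player counts.
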(event `UpdateServer_Fail`
  (`KismetSystemLibrary.PrintString` (`VaRestRequestJSON.ResponseContent` (`VaRestParseManager.ConstructParseRequest` "PUT" "json"))))

(event `UpdateServer_Complete`
  (`KismetSystemLibrary.PrintString` (`VaRestRequestJSON.ResponseContent` (`VaRestParseManager.ConstructParseRequest` "PUT" "json"))))