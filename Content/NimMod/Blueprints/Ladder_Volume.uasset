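; Ladder volume actor that lets a NimModCharacter climb by changing its movement mode while it overlaps the volume.
; On begin overlap, the authority switches the character to Flying and adds a single movement input along its up vector, scaled by LadderMove.
; On end overlap, the authority sets the character back to Walking.
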(event `self.ReceiveActorBeginOverlap`
  (params (OtherActor :type "Actor Object Reference"))
  (`/Engine/EditorBlueprintResources/ActorMacros.Switch Has Authority`
    (:`Authority`
      (bind _asnim_mod_character (cast `NimModCharacter` OtherActor))
      (`CharacterMovementComponent.SetMovementMode` (`Character.CharacterMovement` _asnim_mod_character) "MOVE_Flying" 0)
      (`Pawn.AddMovementInput` _asnim_mod_character (`self.GetActorUpVector` _asnim_mod_character) (`self.LadderMove`) false))))

(event `self.ReceiveActorEndOverlap`
  (params (OtherActor :type "Actor Object Reference"))
  (`/Engine/EditorBlueprintResources/ActorMacros.Switch Has Authority`
    (:`Authority`
      (bind _asnim_mod_character (cast `NimModCharacter` OtherActor))
      (`CharacterMovementComponent.SetMovementMode` (`Character.CharacterMovement` _asnim_mod_character) "MOVE_Walking" 0))))

(fn `UserConstructionScript`)